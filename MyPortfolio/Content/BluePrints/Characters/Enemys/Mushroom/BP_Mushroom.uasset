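; Mushroom enemy Blueprint that turns attack starts from its CombatAttackComponent into attack animation.
; On BeginPlay it caches the component's attack names, and each attack plays the montage matching the first name through BaseAnimInstance.
; The attack ends on the component when that montage ends, interrupted or not, or immediately if the montage fails to play.
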(event OnAttackStarted(CombatAttackComponent)
  (bind _returnvalue (Class|BaseAnimInstance|PlayMontagebyName (Variables|Default|GetBaseAnimInstance) (Utilities|Array|Get(acopy) (Variables|Default|GetAttack%20Names))))
  (if _returnvalue
    (EventDispatchers|BindEventtoOnMontageEnded (Variables|Default|GetBaseAnimInstance) (delegate Custom|EndAttack))
    (else
      (Class|AttackComponent|EndAttack (Variables|Default|GetCombatAttackComponent)))))

(event Custom|EndAttack
  (params (Montage :type Anim%20Montage%20Object%20Reference) (bInterrupted :type Boolean))
  (Class|AttackComponent|EndAttack (Variables|Default|GetCombatAttackComponent)))

(event EventBeginPlay
  (Variables|Default|SetAttack%20Names (Variables|/Script/MyPortfolio.AttackComponent|GetAttackNames (Variables|Default|GetCombatAttackComponent))))

(fn ConstructionScript)
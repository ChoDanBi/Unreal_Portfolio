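; BP_GrapHook is a player component for a grappling hook, currently containing only target detection with debug output.
; It caches the player pawn and camera on BeginPlay, re-fetching the camera on Tick if invalid.
; While the player's action state is Zooming, it line-traces forward from the camera on the Visibility channel each frame, drawing the trace and printing the hit actor.
; No hook firing or pull movement is implemented.
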(event EventBeginPlay
  (bind _output_get (Variables|Default|SetPlayer (.AsMy%20Player (Utilities|Casting|CastToMyPlayer (Game|Player|GetPlayerPawn 0)))))
  (Variables|Default|SetPlayerCamera (Class|MyPlayer|GetCamera _output_get)))

(event EventTick
  (params (DeltaSeconds :type Float%20%28single-precision%29))
  (Utilities|IsValid (Variables|Default|GetPlayerCamera)
    (:Is%20Valid
      _)
    (:Is%20Not%20Valid
      (Variables|Default|SetPlayerCamera (Class|MyPlayer|GetCamera (Variables|Default|GetPlayer)))))
  (if (Utilities|Enum|Equal(Enum) (Class|MyPlayer|GetActionState (Variables|Default|GetPlayer)) (Variables|Default|GetZooming))
    (bind _outhit (Collision|LineTraceByChannel (Transformation|GetWorldLocation (Variables|Default|GetPlayerCamera)) (+ (Transformation|GetWorldLocation (Variables|Default|GetPlayerCamera)) (* (Math|Vector|GetForwardVector (Variables|Default|GetPlayerCamera)) 2e+03)) "TraceTypeQuery1" false 0 "ForDuration" true "(R=1.000000,G=0.000000,B=0.000000,A=1.000000)" "(R=0.000000,G=1.000000,B=0.000000,A=1.000000)" DeltaSeconds))
    (Development|PrintText (Utilities|Text|ToText(Object) (.HitActor (Collision|BreakHitResult _outhit))))))